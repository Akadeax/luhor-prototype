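; BP_StateStun is the player's stun state, which holds until hit stun ends and then returns the player to Locomotion.
; On enter it binds to the hit stun end event of the character's Hittable, and on exit it unbinds.
; When that event fires, it asks the state machine to change to Locomotion.
; It declares a HittableComponent dependency and lazily caches the owner cast to BP_PlayerCharacter.
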(event `self.OnEnterState`
  (add `HittableComponent.OnHitStunEnd` (`/Game/Player/BP_PlayerCharacter.Hittable` (`self.GetCharacter`)) (`|CreateDelegate` :!event `OnHitStunEnd`)))

(event `self.OnExitState`
  (remove `HittableComponent.OnHitStunEnd` (`/Game/Player/BP_PlayerCharacter.Hittable` (`self.GetCharacter`)) (`|CreateDelegate` :!event `OnHitStunEnd`)))

(event `OnHitStunEnd`
  (`StateMachineComponent.TryChangeState` (`self.GetStateMachine`) "Locomotion"))

(fn `GetCharacter`
  (returns (Character :type "/Game/Player/BP_PlayerCharacter Object Reference"))
  (`/Engine/EditorBlueprintResources/StandardMacros.IsValid` (`self.Character`)
    (:`Is Valid`
      _)
    (:`Is Not Valid`
      (bind _asbp_player_character (cast `/Game/Player/BP_PlayerCharacter` (`self.GetOwner`)))
      (set `self.Character` _asbp_player_character)))
  (return (`self.Character`)))

(fn `GetDependencies`
  (returns (ReturnValue :type "Array of ComponentDependency Structure"))
  (return (`|MakeArray` (make `ComponentDependency` "AnyOnActor" "/Script/LuhorPrototype.HittableComponent"))))