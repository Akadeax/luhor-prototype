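; Player state for the secondary melee attack that rate-limits entry with a cooldown.
; Tick counts the remaining cooldown down, and CanEnterState refuses entry until it runs out, then defers to the parent check.
; A passing check restarts the cooldown inside CanEnterState itself, so the query has a side effect.
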(event `self.ReceiveTick`
  (params (DeltaSeconds :type "Float (single-precision)"))
  (if (> (`self.AttackCooldownLeft`) 0.0)
    (set `self.AttackCooldownLeft` (- (`self.AttackCooldownLeft`) DeltaSeconds))))

(fn `CanEnterState`
  (returns (ReturnValue :type Boolean))
  (if (<= (`self.AttackCooldownLeft`) 0.0)
    (bind _returnvalue (`parent.CanEnterState`))
    (if _returnvalue
      (if true
        (set `self.AttackCooldownLeft` (`self.AttackCooldown`))
        (return _returnvalue))
      (else
        (return _returnvalue)))
    (else
      (return false))))

(fn `GetDependencies`
  (returns (ReturnValue :type "Array of ComponentDependency Structure"))
  (return))