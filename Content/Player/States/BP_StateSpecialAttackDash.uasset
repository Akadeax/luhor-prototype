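; Player state for the dash special attack, gating entry on a cooldown and a special charge from an Ambrosia tank.
; Tick counts the cooldown down, and the tank reference arrives through the SetAmbrosiaTank event.
; CanEnterState spends a charge once the cooldown expires, then defers to the parent check and restarts the cooldown only if that passes.
; The charge is spent before the parent check, so a parent refusal still consumes it.
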(event `SetAmbrosiaTank`
  (params (`Ambrosia tank` :type "AmbrosiaHealthComponent Object Reference"))
  (set `self.AmbrosiaContainer` `Ambrosia tank`))

(event `self.ReceiveTick`
  (params (DeltaSeconds :type "Float (single-precision)"))
  (if (> (`self.AttackCooldownLeft`) 0.0)
    (set `self.AttackCooldownLeft` (- (`self.AttackCooldownLeft`) DeltaSeconds))))

(fn `CanEnterState`
  (returns (ReturnValue :type Boolean))
  (if (<= (`self.AttackCooldownLeft`) 0.0)
    (bind _returnvalue (`AmbrosiaHealthComponent.TrySpendSpecialCharge` (`self.AmbrosiaContainer`)))
    (if _returnvalue
      (bind _returnvalue_2 (`parent.CanEnterState`))
      (if _returnvalue_2
        (set `self.AttackCooldownLeft` (`self.AttackCooldown`)))
      (return _returnvalue_2)
      (else
        _)))
  (return false))

(fn `GetDependencies`
  (returns (ReturnValue :type "Array of ComponentDependency Structure"))
  (return))