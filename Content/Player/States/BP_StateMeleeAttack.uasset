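; Player state machine state that runs melee attacks through a child MeleeAttackerComponent.
; Entry is allowed only if the attacker's TryAttack succeeds; while active it listens for attack end, move input and hit stun.
; When an attack ends with another queued, it turns control rotation toward the latest move input, otherwise it returns to locomotion.
; Hit stun also requests locomotion, and exiting unbinds events and cancels the attack.
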(event `self.ReceiveBeginPlay`
  (set `self.Attacker` (`self.GetChildComponentByClass` "/Script/LuhorPrototype.MeleeAttackerComponent")))

(event `self.OnEnterState`
  (add `BaseAttackerComponent.OnAttackDone` (`self.Attacker`) (`|CreateDelegate` :!event `OnAttackEnd`))
  (add `/Game/Player/BP_PlayerCharacter.OnInputMoveTriggered` (`self.GetCharacter`) (`|CreateDelegate` :!event `OnInputMoveTriggered`))
  (add `HittableComponent.OnHitStun` (`/Game/Player/BP_PlayerCharacter.Hittable` (`self.GetCharacter`)) (`|CreateDelegate` :!event `OnHitStun`)))

(event `self.OnExitState`
  (remove `BaseAttackerComponent.OnAttackDone` (`self.Attacker`) (`|CreateDelegate` :!event `OnAttackEnd`))
  (remove `/Game/Player/BP_PlayerCharacter.OnInputMoveTriggered` (`self.GetCharacter`) (`|CreateDelegate` :!event `OnInputMoveTriggered`))
  (remove `HittableComponent.OnHitStun` (`/Game/Player/BP_PlayerCharacter.Hittable` (`self.GetCharacter`)) (`|CreateDelegate` :!event `OnHitStun`))
  (`MeleeAttackerComponent.CancelAttack` (`self.Attacker`)))

(event `OnAttackEnd`
  (bind (_currentmoveinput_x _currentmoveinput_y) (`KismetMathLibrary.BreakVector2D` (`self.CurrentMoveInput`)))
  (if (`MeleeAttackerComponent.IsAttackQueued` (`self.Attacker`))
    (`LuhorCharacter.SetControlRotationFromInputDir` (`self.GetCharacter`) (`KismetMathLibrary.MakeVector` _currentmoveinput_x _currentmoveinput_y) 90.0)
    (else
      (`StateMachineComponent.TryChangeState` (`self.GetStateMachine`) "locomotion"))))

(event `OnInputMoveTriggered`
  (params (Input :type "Vector2D Structure"))
  (set `self.CurrentMoveInput` Input))

(event `OnHitStun`
  (`StateMachineComponent.TryChangeState` (`self.GetStateMachine`) "Locomotion"))

(fn `CanEnterState`
  (returns (ReturnValue :type Boolean))
  (bind _returnvalue (`MeleeAttackerComponent.TryAttack` (`self.Attacker`)))
  (return _returnvalue))

(fn `GetCharacter`
  (returns (Character :type "/Game/Player/BP_PlayerCharacter Object Reference"))
  (`/Engine/EditorBlueprintResources/StandardMacros.IsValid` (`self.Character`)
    (:`Is Valid`
      _)
    (:`Is Not Valid`
      (bind _asbp_player_character (cast `/Game/Player/BP_PlayerCharacter` (`self.GetOwner`)))
      (set `self.Character` _asbp_player_character)))
  (return (`self.Character`)))

(fn `GetDependencies`
  (returns (ReturnValue :type "Array of ComponentDependency Structure"))
  (return (`|MakeArray` (make `ComponentDependency` "Child" "/Script/LuhorPrototype.MeleeAttackerComponent"))))