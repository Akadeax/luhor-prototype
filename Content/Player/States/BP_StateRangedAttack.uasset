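; Player state machine state for aiming and firing the gun, enterable only when the attacker is ready and a bullet remains.
; While aiming, move input steers rotation, with angular aim assist snapping to enemies in unobstructed line of sight.
; A Niagara beam previews the shot, clipped by a line trace.
; Shooting spends a bullet and freezes aim; attack completion returns to Locomotion, while hit stun switches to Stun.
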(event `self.ReceiveBeginPlay`
  (set `self.Attacker` (`self.GetChildComponentByClass` "/Script/LuhorPrototype.RangedAttackerComponent"))
  (set `self.AimPreview` (`self.GetChildComponentByClass` "/Script/Niagara.NiagaraComponent"))
  (`self.DisablePreview`)
  (set `self.GunComponent` (`Actor.GetComponentByClass` (`self.GetOwner`) "/Game/Player/Ranged/BP_GunComponent.BP_GunComponent_C")))

(event `self.OnEnterState`
  (set `self.Aiming` true)
  (`self.EnablePreview`)
  (add `BaseAttackerComponent.OnAttackDone` (`self.Attacker`) (`|CreateDelegate` :!event `OnAttackDone`))
  (add `HittableComponent.OnHitStun` (`/Game/Player/BP_PlayerCharacter.Hittable` (`self.GetCharacter`)) (`|CreateDelegate` :!event `OnHitStun`))
  (add `/Game/Player/BP_PlayerCharacter.OnInputRangedAttackShoot` (`self.GetCharacter`) (`|CreateDelegate` :!event `OnRangedAttackShoot`))
  (add `/Game/Player/BP_PlayerCharacter.OnInputMoveTriggered` (`self.GetCharacter`) (delegate `OnMoveInput`))
  (`self.SetDirFromRotation`))

(event `self.OnExitState`
  (bind _attacker (`self.Attacker`))
  (`RangedAttackerComponent.CancelAttack` _attacker)
  (remove `BaseAttackerComponent.OnAttackDone` _attacker (`|CreateDelegate` :!event `OnAttackDone`))
  (remove `HittableComponent.OnHitStun` (`/Game/Player/BP_PlayerCharacter.Hittable` (`self.GetCharacter`)) (`|CreateDelegate` :!event `OnHitStun`))
  (remove `/Game/Player/BP_PlayerCharacter.OnInputRangedAttackShoot` (`self.GetCharacter`) (`|CreateDelegate` :!event `OnRangedAttackShoot`))
  (remove `/Game/Player/BP_PlayerCharacter.OnInputMoveTriggered` (`self.GetCharacter`) (delegate `OnMoveInput`))
  (`self.DisablePreview`))

(event `OnMoveInput`
  (params (Input :type "Vector2D Structure"))
  (set `self.CurrentMoveInput` (`KismetMathLibrary.Normal2D` Input)))

(event `OnHitStun`
  (`StateMachineComponent.TryChangeState` (`self.GetStateMachine`) "Stun"))

(event `OnAttackDone`
  (`StateMachineComponent.TryChangeState` (`self.GetStateMachine`) "Locomotion"))

(event `OnRangedAttackShoot`
  (bind _returnvalue (`RangedAttackerComponent.TryAttack` (`self.Attacker`)))
  (if _returnvalue
    (set `self.Aiming` false)
    (`self.DisablePreview`)
    (`/Game/Player/Ranged/BP_GunComponent.UseBullet` (`self.GunComponent`))))

(event `self.OnUpdateState`
  (if (`self.Aiming`)
    (`self.DoRotation`)
    (`self.CheckAimPreview`)))

(event `EnablePreview`
  (`self.SetHiddenInGame` (`self.AimPreview`) false false))

(event `DisablePreview`
  (`self.SetHiddenInGame` (`self.AimPreview`) true false))

(fn `CanEnterState`
  (returns (ReturnValue :type Boolean))
  (return (and (`BaseAttackerComponent.CanAttack` (`self.Attacker`)) (`/Game/Player/Ranged/BP_GunComponent.HasBullet` (`self.GunComponent`)))))

(fn `CheckAimPreview`
  (locals (BeamStart :type "Vector Structure") (BeamEnd :type "Vector Structure"))
  (bind _output_get (set `local.BeamStart` (`self.K2_GetComponentLocation` (`self.Attacker`))))
  (`NiagaraComponent.SetVariablePosition` (`self.AimPreview`) "BeamStart" _output_get)
  (bind _output_get_2 (set `local.BeamEnd` (+ (`local.BeamStart`) (* (`Actor.GetActorForwardVector` (`self.GetCharacter`)) 10000.0))))
  (bind (_outhit _returnvalue) (`KismetSystemLibrary.LineTraceSingle` (`local.BeamStart`) _output_get_2 "TraceTypeQuery3"))
  (bind (_bblockinghit _binitialoverlap _time _distance _location _impactpoint _normal _impactnormal _physmat _hitactor _hitcomponent _hitbonename _bonename _hititem _elementindex _faceindex _tracestart _traceend) (`GameplayStatics.BreakHitResult` _outhit))
  (`NiagaraComponent.SetVariableVec3` (`self.AimPreview`) "BeamEnd" (`KismetMathLibrary.SelectVector` _location _traceend _returnvalue)))

(fn `DoRotation`
  (locals (InputYaw :type "Float (double-precision)") (AnyAimAssist :type Boolean))
  (bind _aimassistdegrees (`self.AimAssistDegrees`))
  (bind (_x _y) (`KismetMathLibrary.BreakVector2D` (`self.CurrentMoveInput`)))
  (set `local.InputYaw` (`KismetMathLibrary.DegAtan2` _x _y))
  (bind _enemies (`self.GetEnemiesInLOS`))
  (for _array_element _enemies
    (bind _returnvalue (- (`Actor.K2_GetActorLocation` _array_element) (`Actor.K2_GetActorLocation` (`self.GetCharacter`))))
    (bind _returnvalue_2 (`KismetMathLibrary.Abs` (- (`KismetMathLibrary.DegAtan2` (.y _returnvalue) (.x _returnvalue)) (`local.InputYaw`))))
    (if (or (> _returnvalue_2 (- 360.0 _aimassistdegrees)) (< _returnvalue_2 _aimassistdegrees))
      (`LuhorCharacter.SetControlRotationFromInputDir` (`self.GetCharacter`) (`KismetMathLibrary.MakeVector` (.y (`KismetMathLibrary.Normal` _returnvalue)) (.x (`KismetMathLibrary.Normal` _returnvalue))) 90.0)
      (set `local.AnyAimAssist` true)))
  (if (not (`local.AnyAimAssist`))
    (`LuhorCharacter.SetControlRotationFromInputDir` (`self.GetCharacter`) (`KismetMathLibrary.Conv_Vector2DToVector` (`self.CurrentMoveInput`)) 90.0)))

(fn `GetCharacter`
  (returns (Character :type "/Game/Player/BP_PlayerCharacter Object Reference"))
  (`/Engine/EditorBlueprintResources/StandardMacros.IsValid` (`self.Character`)
    (:`Is Valid`
      _)
    (:`Is Not Valid`
      (bind _asbp_player_character (cast `/Game/Player/BP_PlayerCharacter` (`self.GetOwner`)))
      (set `self.Character` _asbp_player_character)))
  (return (`self.Character`)))

(fn `GetDependencies`
  (returns (ReturnValue :type "Array of ComponentDependency Structure"))
  (return (`|MakeArray` (make `ComponentDependency` "Child" "/Script/LuhorPrototype.RangedAttackerComponent") (make `ComponentDependency` "Child" "/Script/Niagara.NiagaraComponent"))))

(fn `GetEnemiesInLOS`
  (returns (Enemies :type "Array of LuhorEnemyCharacter Object Reference"))
  (locals (En :type "Array of LuhorEnemyCharacter Object Reference"))
  (bind _outactors (`GameplayStatics.GetAllActorsOfClass` "/Script/LuhorPrototype.LuhorEnemyCharacter"))
  (for _array_element _outactors
    (bind (_outhit _returnvalue) (`KismetSystemLibrary.LineTraceSingle` (`Actor.K2_GetActorLocation` (`self.GetCharacter`)) (`Actor.K2_GetActorLocation` _array_element) "TraceTypeQuery3"))
    (if (not _returnvalue)
      (`KismetArrayLibrary.Array_Add` (`local.En`) _array_element)))
  (return (`local.En`)))

(fn `SetDirFromRotation`
  (bind _returnvalue (`KismetMathLibrary.DegreesToRadians` (.yaw (`Pawn.GetControlRotation` (`self.GetCharacter`)))))
  (set `self.CurrentMoveInput` (`KismetMathLibrary.MakeVector2D` (`KismetMathLibrary.Sin` _returnvalue) (`KismetMathLibrary.Cos` _returnvalue))))