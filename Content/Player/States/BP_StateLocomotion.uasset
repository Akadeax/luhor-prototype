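; BP_StateLocomotion is the player's locomotion state in a state machine, handling movement and transitions into attack or stun.
; On enter it binds to the player character's move, attack and hit-stun events, and unbinds them on exit.
; Move input drives movement and control rotation, while attack and hit-stun events request melee attack or Stun states.
; GetCharacter lazily casts and caches the owning BP_PlayerCharacter.
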(event `self.OnEnterState`
  (add `/Game/Player/BP_PlayerCharacter.OnInputMoveTriggered` (`self.GetCharacter`) (`|CreateDelegate` :!event `OnInputMoveTriggered`))
  (add `/Game/Player/BP_PlayerCharacter.OnInputMoveCompleted` (`self.GetCharacter`) (`|CreateDelegate` :!event `OnInputMoveComplete`))
  (add `/Game/Player/BP_PlayerCharacter.OnInputPrimaryAttackTriggered` (`self.GetCharacter`) (`|CreateDelegate` :!event `OnInputPrimaryAttackTriggered`))
  (add `/Game/Player/BP_PlayerCharacter.OnInputSecondaryAttackTriggered` (`self.GetCharacter`) (`|CreateDelegate` :!event `OnInputSecondaryAttackTriggered`))
  (add `HittableComponent.OnHitStun` (`/Game/Player/BP_PlayerCharacter.Hittable` (`self.GetCharacter`)) (`|CreateDelegate` :!event `OnHitStun`)))

(event `self.OnExitState`
  (remove `/Game/Player/BP_PlayerCharacter.OnInputMoveTriggered` (`self.GetCharacter`) (`|CreateDelegate` :!event `OnInputMoveTriggered`))
  (remove `/Game/Player/BP_PlayerCharacter.OnInputMoveCompleted` (`self.GetCharacter`) (`|CreateDelegate` :!event `OnInputMoveComplete`))
  (remove `/Game/Player/BP_PlayerCharacter.OnInputPrimaryAttackTriggered` (`self.GetCharacter`) (`|CreateDelegate` :!event `OnInputPrimaryAttackTriggered`))
  (remove `/Game/Player/BP_PlayerCharacter.OnInputSecondaryAttackTriggered` (`self.GetCharacter`) (`|CreateDelegate` :!event `OnInputSecondaryAttackTriggered`))
  (remove `HittableComponent.OnHitStun` (`/Game/Player/BP_PlayerCharacter.Hittable` (`self.GetCharacter`)) (`|CreateDelegate` :!event `OnHitStun`)))

(event `OnInputMoveTriggered`
  (params (Input :type "Vector2D Structure"))
  (bind (_currentinput_x _currentinput_y) (`KismetMathLibrary.BreakVector2D` (`self.CurrentInput`)))
  (bind _output_get (set `self.CurrentInput` Input))
  (bind (_x _y) (`KismetMathLibrary.BreakVector2D` _output_get))
  (`Pawn.AddMovementInput` (`self.GetCharacter`) (`KismetMathLibrary.MakeVector` _y _x) 1.0 false)
  (`LuhorCharacter.SetControlRotationFromInputDir` (`self.GetCharacter`) (`KismetMathLibrary.MakeVector` _currentinput_x _currentinput_y) 90.0))

(event `OnInputMoveComplete`
  (set `self.CurrentInput` (0.0 0.0)))

(event `OnInputPrimaryAttackTriggered`
  (`StateMachineComponent.TryChangeState` (`self.GetStateMachine`) "MeleeAttackPrimary"))

(event `OnInputSecondaryAttackTriggered`
  (`StateMachineComponent.TryChangeState` (`self.GetStateMachine`) "MeleeAttackSecondary"))

(event `OnHitStun`
  (`StateMachineComponent.TryChangeState` (`self.GetStateMachine`) "Stun"))

(fn `GetCharacter`
  (returns (Character :type "/Game/Player/BP_PlayerCharacter Object Reference"))
  (`/Engine/EditorBlueprintResources/StandardMacros.IsValid` (`self.Character`)
    (:`Is Valid`
      _)
    (:`Is Not Valid`
      (bind _asbp_player_character (cast `/Game/Player/BP_PlayerCharacter` (`self.GetOwner`)))
      (set `self.Character` _asbp_player_character)))
  (return (`self.Character`)))