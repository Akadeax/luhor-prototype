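; BP_GhostUpgrade is a player upgrade Blueprint that recolors the player's sword trail while the player is empowered.
; On empower start it casts PlayerCharacter to BP_PlayerCharacter and sets the sword trail effect's TrailColor parameter to a bright HDR purple.
; On empower end it sets the same parameter to an orange color.
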(event `self.OnEmpowerStart`
  (bind _asbp_player_character (cast `/Game/Player/BP_PlayerCharacter` (`self.PlayerCharacter`)))
  (`NiagaraComponent.SetVariableLinearColor` (`/Game/Player/BP_PlayerCharacter.FXS_Sword_Trail` _asbp_player_character) "TrailColor" (`KismetMathLibrary.MakeColor` 4.75 0.1 10.0)))

(event `self.OnEmpowerEnd`
  (bind _asbp_player_character (cast `/Game/Player/BP_PlayerCharacter` (`self.PlayerCharacter`)))
  (`NiagaraComponent.SetVariableLinearColor` (`/Game/Player/BP_PlayerCharacter.FXS_Sword_Trail` _asbp_player_character) "TrailColor" (`KismetMathLibrary.MakeColor` 10.0 4.8)))