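; Player character built on an Ambrosia health pool, which is wired into the special AOE and dash attacks and siphoned from melee hit damage.
; Tick scales drain VFX and lamp lights by health, while attack and last-stand events recolor, burst or hide effects.
; Enhanced Input relays movement and attacks and triggers overlapping interactables; Tab grants debug god mode.
; Death resets upgrades, health and rooms, then reloads Main; helpers define curve-driven knockback.
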(event Custom|OnDeath
  (Class|UpgradesComponent|ClearUpgrades (Variables|Default|GetUpgrades))
  (Class|HealthComponent|Heal (Variables|Default|GetAmbrosiaHealth) 2e+02)
  (Class|LevelGameInstanceSubsystem|RefillRoomsLeft (Subsystems|GetLevelGameInstanceSubsystem))
  (Class|UpgradesComponent|ClearUpgrades (Variables|Default|GetUpgrades))
  (Class|AmbrosiaHealthComponent|ResetBools (Variables|Default|GetAmbrosiaHealth))
  (Game|OpenLevel(byObjectReference) "/Game/Main.Main"))

(event Custom|OnSiphon
  (params (Data :type Hittable%20Hit%20Data%20Structure) (WasLethal :type Boolean))
  (Class|AmbrosiaHealthComponent|SiphonAmbrosia (Variables|Default|GetAmbrosiaHealth) (.Damage (Utilities|Struct|BreakHittableHitData Data))))

(event Custom|OnSpecialAttackStarted
  (bind _ambrosiadrain (Variables|Default|GetAmbrosiaDrain))
  (Effects|Components|ParticleSystem|SetColorParameter _ambrosiadrain "Poison" "(R=0.269565,G=0.073482,B=0.556522,A=1.000000)")
  (Niagara|ReinitializeSystem _ambrosiadrain))

(event Custom|OnSpecialAOEStarted
  (Components|Activation|Activate (Variables|Default|GetAOE_Burst) true))

(event Custom|OnSpecialAttackEnded
  (bind _ambrosiadrain (Variables|Default|GetAmbrosiaDrain))
  (Effects|Components|ParticleSystem|SetColorParameter _ambrosiadrain "ambrosia" "(R=1.000000,G=0.681360,B=0.147826,A=1.000000)")
  (Niagara|ReinitializeSystem _ambrosiadrain))

(event Custom|OnLastStandStarted
  (bind _ambrosiadrain (Variables|Default|GetAmbrosiaDrain))
  (Class|NiagaraComponent|SetPaused _ambrosiadrain true)
  (Rendering|SetVisibility _ambrosiadrain false false))

(event Custom|OnLastStandEnded
  (bind _ambrosiadrain (Variables|Default|GetAmbrosiaDrain))
  (Class|NiagaraComponent|SetPaused _ambrosiadrain false)
  (Rendering|SetVisibility _ambrosiadrain true false))

(event Input|EnhancedActionEvents|EnhancedInputActionIA_Move
  (params (ActionValue :type Vector%202D%20Structure) (ElapsedSeconds :type Float%20%28double-precision%29) (TriggeredSeconds :type Float%20%28double-precision%29) (InputAction :type Input%20Action%20Object%20Reference :default "/Game/Player/Input/IA_Move.IA_Move"))
  (bind _returnvalue (Class|KismetMathLibrary|VSize2DSquared ActionValue))
  (bind _returnvalue_2 (> _returnvalue 0.1))
  (:Triggered
    (if _returnvalue_2
      (Default|CallOnInputMoveTriggered ActionValue)))
  (:Completed
    (if _returnvalue_2
      (Default|CallOnInputMoveCompleted))))

(event Input|EnhancedActionEvents|EnhancedInputActionIA_PrimaryAttack
  (params (ActionValue :type Boolean) (ElapsedSeconds :type Float%20%28double-precision%29) (TriggeredSeconds :type Float%20%28double-precision%29) (InputAction :type Input%20Action%20Object%20Reference :default "/Game/Player/Input/IA_PrimaryAttack.IA_PrimaryAttack"))
  (Default|CallOnInputPrimaryAttackTriggered))

(event Input|EnhancedActionEvents|EnhancedInputActionIA_SecondaryAttack
  (params (ActionValue :type Boolean) (ElapsedSeconds :type Float%20%28double-precision%29) (TriggeredSeconds :type Float%20%28double-precision%29) (InputAction :type Input%20Action%20Object%20Reference :default "/Game/Player/Input/IA_SecondaryAttack.IA_SecondaryAttack"))
  (Default|CallOnInputSecondaryAttackTriggered))

(event Input|EnhancedActionEvents|EnhancedInputActionIA_Interract
  (params (ActionValue :type Boolean) (ElapsedSeconds :type Float%20%28double-precision%29) (TriggeredSeconds :type Float%20%28double-precision%29) (InputAction :type Input%20Action%20Object%20Reference :default "/Game/Player/Input/IA_Interract.IA_Interract"))
  (bind _self self)
  (for _array_element (Collision|GetOverlappingActors (Variables|Default|GetCapsuleComponent) "/Script/Engine.Actor" :!class /Script/Engine.PrimitiveComponent)
    (if (Utilities|DoesObjectImplementInterface _array_element "/Script/LuhorPrototype.Interactable")
      (bind _returnvalue (Class|Interactable|CanInteract(Message) _array_element _self))
      (if _returnvalue
        (Class|Interactable|Interact(Message) _array_element _self)))))

(event Input|EnhancedActionEvents|EnhancedInputActionIA_SpecialDashAttack
  (params (ActionValue :type Boolean) (ElapsedSeconds :type Float%20%28double-precision%29) (TriggeredSeconds :type Float%20%28double-precision%29) (InputAction :type Input%20Action%20Object%20Reference :default "/Game/Player/Input/IA_SpecialDashAttack.IA_SpecialDashAttack"))
  (Default|CallOnInputSpecialDashAttackTriggered))

(event Input|EnhancedActionEvents|EnhancedInputActionIA_SpecialAOEAttack
  (params (ActionValue :type Boolean) (ElapsedSeconds :type Float%20%28double-precision%29) (TriggeredSeconds :type Float%20%28double-precision%29) (InputAction :type Input%20Action%20Object%20Reference :default "/Game/Player/Input/IA_SpecialAOEAttack.IA_SpecialAOEAttack"))
  (Default|CallOnInputSpecialAOEAttackTriggered))

(event Input|EnhancedActionEvents|EnhancedInputActionIA_RangedAttackAim
  (params (ActionValue :type Boolean) (ElapsedSeconds :type Float%20%28double-precision%29) (TriggeredSeconds :type Float%20%28double-precision%29) (InputAction :type Input%20Action%20Object%20Reference :default "/Game/Player/Input/IA_RangedAttackAim.IA_RangedAttackAim"))
  (Default|CallOnInputRangedAttackAim))

(event Input|EnhancedActionEvents|EnhancedInputActionIA_RangedAttackShoot
  (params (ActionValue :type Boolean) (ElapsedSeconds :type Float%20%28double-precision%29) (TriggeredSeconds :type Float%20%28double-precision%29) (InputAction :type Input%20Action%20Object%20Reference :default "/Game/Player/Input/IA_RangedAttackShoot.IA_RangedAttackShoot"))
  (Default|CallOnInputRangedAttackShoot))

(event EventTick
  (params (DeltaSeconds :type Float%20%28single-precision%29))
  (bind _maxambrosialightintensity (Variables|Default|GetMaxAmbrosiaLightIntensity))
  (bind _ambrosialightfloor (Variables|Default|GetAmbrosiaLightFloor))
  (bind _ambrosiahealth (Variables|Default|GetAmbrosiaHealth))
  (bind _returnvalue (Class|HealthComponent|GetCurrentHealth _ambrosiahealth))
  (bind _returnvalue_2 (Class|HealthComponent|GetMaxHealth _ambrosiahealth))
  (bind _returnvalue_3 (/ _returnvalue _returnvalue_2))
  (bind _returnvalue_4 (* _maxambrosialightintensity _returnvalue_3))
  (bind _returnvalue_5 (Math|Float|Max(Float) _returnvalue_4 _ambrosialightfloor))
  (Effects|Components|ParticleSystem|SetFloatParameter (Variables|Default|GetAmbrosiaDrain) "Health_Div" _returnvalue_3)
  (Rendering|Components|Light|SetIntensity (Variables|Default|GetAmbrosiaLamp) _returnvalue_5)
  (Rendering|Components|Light|SetIntensity (Variables|Default|GetAmbrosiaLampPlayerRim) (/ _returnvalue_5 2.0)))

(event EventBeginPlay
  (bind _ambrosiahealth (Variables|Default|GetAmbrosiaHealth))
  (bind _specialaoemeleeattacker (Variables|Default|GetSpecialAOEMeleeAttacker))
  (bind _specialdashmeleeattacker (Variables|Default|GetSpecialDashMeleeAttacker))
  (bind _ambrosiahealth_2 (Variables|Default|GetAmbrosiaHealth))
  (Utilities|FlowControl|Sequence
    (:then_0
      (Transformation|AttachComponentToComponent (Variables|Default|Getsword) (Variables|Character|GetMesh) "Weapon" "SnapToTarget" "SnapToTarget" "KeepRelative" false)
      (bind _returnvalue (Game|ConstructObjectfromClass "/Game/Player/UI/WBP_PlayerHealthBar.WBP_PlayerHealthBar_C" (Variables|Default|GetAmbrosiaHealth)))
      (UserInterface|Viewport|AddtoViewport _returnvalue 0))
    (:then_1
      (Default|SetAmbrosiaTank (Variables|Default|GetSpecialAttackAOE) _ambrosiahealth)
      (Default|SetAmbrosiaTank (Variables|Default|GetSpecialAttackDash) _ambrosiahealth))
    (:then_2
      (EventDispatchers|AssignOnMeleeAttackHit (Variables|Default|GetPrimaryMeleeAttacker) (EventDispatchers|CreateEvent :!event Custom|OnSiphon))
      (EventDispatchers|AssignOnMeleeAttackHit (Variables|Default|GetSecondaryMeleeAttacker) (EventDispatchers|CreateEvent :!event Custom|OnSiphon)))
    (:then_3
      (EventDispatchers|BindEventtoOnAttackDone _specialaoemeleeattacker (EventDispatchers|CreateEvent :!event Custom|OnSpecialAttackEnded))
      (EventDispatchers|BindEventtoOnAttackStarted _specialaoemeleeattacker (EventDispatchers|CreateEvent :!event Custom|OnSpecialAttackStarted))
      (EventDispatchers|BindEventtoOnAttackStarted _specialaoemeleeattacker (EventDispatchers|CreateEvent :!event Custom|OnSpecialAOEStarted))
      (EventDispatchers|BindEventtoOnAttackDone _specialdashmeleeattacker (EventDispatchers|CreateEvent :!event Custom|OnSpecialAttackEnded))
      (EventDispatchers|BindEventtoOnAttackStarted _specialdashmeleeattacker (EventDispatchers|CreateEvent :!event Custom|OnSpecialAttackStarted)))
    (:then_4
      (EventDispatchers|BindEventtoOnLastStandStarted _ambrosiahealth_2 (EventDispatchers|CreateEvent :!event Custom|OnLastStandStarted))
      (EventDispatchers|BindEventtoOnLastStandEnded _ambrosiahealth_2 (EventDispatchers|CreateEvent :!event Custom|OnLastStandEnded)))
    (:then_5
      (EventDispatchers|BindEventtoOnDeath (Variables|Default|GetAmbrosiaHealth) (EventDispatchers|CreateEvent :!event Custom|OnDeath)))))

(event Input|KeyboardEvents|DebugKeyTab
  (params (Key :type Key%20Structure :default "None") (ActionValue :type Input%20Action%20Value%20Structure))
  (:Pressed
    (Class|UpgradesComponent|AddUpgrade (Variables|Default|GetUpgrades) "/Game/Player/Upgrades/BP_GodModeUpgrade.BP_GodModeUpgrade_C")))

(fn ConstructionScript)

(fn Knock
  (params (Time :type Float%20%28double-precision%29) (Dir :type Vector :default "1.000000,0.000000,0.000000") (Force :type Float%20%28double-precision%29) (ForceMultiplierCurve :type Curve%20Float%20Object%20Reference))
  (Variables|Knock|SetKnockTime Time)
  (Variables|Knock|SetKnockDir Dir)
  (Variables|Knock|SetKnockForce Force)
  (Variables|Default|SetKnockForceMultiplierCurve ForceMultiplierCurve)
  (Variables|Knock|SetKnockTimeLeft (Variables|Knock|GetKnockTime)))

(fn HandleKnock
  (params (Delta :type Float%20%28double-precision%29))
  (if (> (Variables|Knock|GetKnockTimeLeft) 0.0)
    (Variables|Knock|SetKnockTimeLeft (- (Variables|Knock|GetKnockTimeLeft) Delta))
    (bind _output_get (LocalVariables|SetCurrentKnockForce (* (Variables|Knock|GetKnockForce) (Math|Curves|GetFloatValue (Variables|Default|GetKnockForceMultiplierCurve) (- 1.0 (/ (Variables|Knock|GetKnockTimeLeft) (Variables|Knock|GetKnockTime)))))))
    (Physics|AddForce (Variables|Character|GetCharacterMovement) (* _output_get (Math|Vector|Normalize (Variables|Knock|GetKnockDir)) 1e+05))
    (if (<= (Variables|Knock|GetKnockTimeLeft) 0.0)
      _)))