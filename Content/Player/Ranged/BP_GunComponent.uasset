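; Gun component for the player character that cycles through ranged attack types as switchable bullets.
; On BeginPlay it finds the owner's RangedAttackerComponent, binds to the player's switch-bullet input event and calls NextBullet once.
; Each switch advances a wrapping index into the Attacks array and passes that entry to the attacker component.
; GetBulletPercentage is a placeholder built on constants that always returns zero.
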(event `self.ReceiveBeginPlay`
  (set `self.RangedAttacker` (`Actor.GetComponentByClass` (`self.GetOwner`) "/Script/LuhorPrototype.RangedAttackerComponent"))
  (bind _asbp_player_character (cast `/Game/Player/BP_PlayerCharacter` (`self.GetOwner`)))
  (bind _output_get (set `self.Player` _asbp_player_character))
  (add `/Game/Player/BP_PlayerCharacter.OnInputSwitchBulletTriggered` _output_get (`|CreateDelegate` :!event `OnSwitchBulletTriggered`))
  (`self.NextBullet`))

(event `OnSwitchBulletTriggered`
  (`self.NextBullet`))

(fn `GetBulletPercentage`
  (returns (Result :type "Float (double-precision)"))
  (if (== 0 0)
    (return (`KismetMathLibrary.Conv_IntToDouble` 0))
    (else
      (return (+ 0.0 (- 1.0 (/ 0.0 0.0)))))))

(fn `IncrementBullet`
  (bind _result (`/Engine/EditorBlueprintResources/StandardMacros.IncrementInt` (`self.CurrentAttackIndex`))
    (:`  `
      (if (== _result (`KismetArrayLibrary.Array_Length` (`self.Attacks`)))
        (set `self.CurrentAttackIndex` 0)))))

(fn `NextBullet`
  (`self.IncrementBullet`)
  (`RangedAttackerComponent.SetRangedAttack` (`self.RangedAttacker`) (`|GetArrayItem` (`self.Attacks`) (`self.CurrentAttackIndex`))))