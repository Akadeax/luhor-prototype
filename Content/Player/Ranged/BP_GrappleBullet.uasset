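; BP_GrappleBullet is a player ranged projectile that pulls the target it hits toward the source of the hit.
; On BeginPlay it binds to the projectile hit event, whose handler requires the target's owner to have health remaining and a LuhorMovementComponent.
; It then calls DoCurvedLaunch on that component with a fixed short time and force, directed from the hit location to the source.
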(event `self.ReceiveBeginPlay`
  (add `self.OnProjectileHit` (`|CreateDelegate` :!event `ProjectileHit`)))

(fn `ProjectileHit`
  (params (Data :type "HittableHitData Structure (by ref)") (WasLethal :type Boolean) (Target :type "HittableComponent Object Reference"))
  (locals (Direction :type "Vector Structure"))
  (bind (_damage _source _targetlocation) (break `HittableHitData` Data))
  (bind _returnvalue (`ActorComponent.GetOwner` Target))
  (`/Engine/EditorBlueprintResources/StandardMacros.IsValid` Target
    (:`Is Valid`
      (bind _output_get (set `self.HealthComponent` (`self.GetComponentByClass` _returnvalue "/Script/LuhorPrototype.HealthComponent")))
      (`/Engine/EditorBlueprintResources/StandardMacros.IsValid` _output_get
        (:`Is Valid`
          (bind _output_get_2 (set `self.MovementComponent` (`self.GetComponentByClass` _returnvalue "/Script/LuhorPrototype.LuhorMovementComponent")))
          (`/Engine/EditorBlueprintResources/StandardMacros.IsValid` _output_get_2
            (:`Is Valid`
              (if (> (`HealthComponent.GetCurrentHealth` (`self.HealthComponent`)) 0.0)
                (bind _output_get_3 (set `local.Direction` (- (`self.K2_GetActorLocation` _source) _targetlocation)))
                (`LuhorMovementComponent.DoCurvedLaunch` (`self.MovementComponent`) _output_get_3 (make `CurvedLaunchData` 0.4))
                (return)))))))))

(fn `UserConstructionScript`)