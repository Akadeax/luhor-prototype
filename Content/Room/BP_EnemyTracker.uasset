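; BP_EnemyTracker is a room actor that keeps the player's Ambrosia health drain active until enemies are cleared.
; On BeginPlay it starts the drain on the player's AmbrosiaHealth and notifies the player character.
; Each Tick it polls for all LuhorEnemyCharacter actors in the world, not just one room.
; When none remain, a DoOnce opens the referenced Door, ends the drain and notifies the player.
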(event `self.ReceiveBeginPlay`
  (bind _asbp_player_character (cast `/Game/Player/BP_PlayerCharacter` (`GameplayStatics.GetPlayerPawn` 0)))
  (`AmbrosiaHealthComponent.StartDrain` (`/Game/Player/BP_PlayerCharacter.AmbrosiaHealth` _asbp_player_character))
  (`/Game/Player/BP_PlayerCharacter.OnDrainEnabled` _asbp_player_character))

(event `self.ReceiveTick`
  (params (DeltaSeconds :type "Float (single-precision)"))
  (bind _outactors (`GameplayStatics.GetAllActorsOfClass` "/Script/LuhorPrototype.LuhorEnemyCharacter"))
  (if (== (`KismetArrayLibrary.Array_Length` _outactors) 0)
    (`/Engine/EditorBlueprintResources/StandardMacros.DoOnce` false
      (:`Completed`
        (`/Game/Room/BP_RoomEndDoor.Open` (`self.Door`))
        (bind _asbp_player_character (cast `/Game/Player/BP_PlayerCharacter` (`GameplayStatics.GetPlayerPawn` 0)))
        (`AmbrosiaHealthComponent.EndDrain` (`/Game/Player/BP_PlayerCharacter.AmbrosiaHealth` _asbp_player_character))
        (`/Game/Player/BP_PlayerCharacter.OnDrainDisabled` _asbp_player_character)))))

(fn `UserConstructionScript`)