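; BP_EnemySpawner is an actor that keeps waves of BP_FastMeleeCharacter enemies coming during combat.
; Every Tick it searches the world for that class and, only when none exist, spawns a new batch in a loop.
; Each spawn lands at a fixed distance from the spawner in a random 3D direction, so height varies too, with collision handling left at default.
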(event `self.ReceiveTick`
  (params (DeltaSeconds :type "Float (single-precision)"))
  (bind _outactors (`GameplayStatics.GetAllActorsOfClass` "/Game/Combat/Enemies/FastMelee/BP_FastMeleeCharacter.BP_FastMeleeCharacter_C"))
  (if (== (`KismetArrayLibrary.Array_Length` _outactors) 0)
    (for _ (range 6)
      (`|SpawnActorFromClass` "/Game/Combat/Enemies/FastMelee/BP_FastMeleeCharacter.BP_FastMeleeCharacter_C" (`KismetMathLibrary.MakeTransform` (+ (.location (`self.GetTransform`)) (* (`KismetMathLibrary.RandomUnitVector`) 500.0))) "Undefined" "MultiplyWithRoot" null null))))

(fn `UserConstructionScript`)